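; Enemy Wendigo is an AI-controlled enemy that damages the first-person player character with a melee attack.
; On BeginPlay it writes its RandomRange value to the blackboard for the AI to use.
; The AttackPlayer event sphere-traces a short distance forward for pawns, with debug drawing on, and applies PlayerDamage when the hit actor is the first-person character.
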(event Custom|Attack%20Player
  (bind _returnvalue (Transformation|GetActorLocation))
  ;[0.277 1 0.992] Custom event functionality for attacking the player where a sphere collision is created from the AI actor, where if they see the player and are in the range of colliding, their health is subtracted by 10. Continuously means a restart of the player's current loop.
  (bind (_outhit _returnvalue_2) (Collision|SphereTraceForObjects _returnvalue (+ _returnvalue (* (Math|Vector|GetForwardVector (Transformation|GetActorRotation)) 2.5e+02)) 1.2e+02 (Utilities|Array|MakeArray "ObjectTypeQuery3") false 0 "ForDuration"))
  (if _returnvalue_2
    (bind _asbp_first_person_character (Utilities|Casting|CastToBP_FirstPersonCharacter (.HitActor (Collision|BreakHitResult _outhit))))
    (Default|TakeDamage _asbp_first_person_character (Variables|Default|GetPlayerDamage))))

(event EventBeginPlay
  ;[0.1557 1 0.4513] Function that calls a blackboard to assign the enemy AI's random movement, as tailored by the RandomRange float variable.
  (AI|Components|Blackboard|SetValueasFloat (AI|GetBlackboard 0) (Utilities|Name|MakeLiteralName "RandomRange") (Variables|Default|GetRandomRange)))

(fn ConstructionScript)