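; Slime monster enemy that roams, chases the player and deals melee damage, driven by Blueprint events without a behaviour tree.
; It loops AI MoveTo to random reachable points around itself from BeginPlay.
; PawnSensing starts a chase on a seen pawn, and a retriggerable delay resumes roaming once sightings stop.
; Collision box overlaps fire a debug-drawn forward sphere trace that applies PlayerDamage to a hit BP_FirstPersonCharacter.
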(event OnSeePawn(PawnSensing)
  (params (Pawn :type Pawn%20Object%20Reference))
  ;[0.1557 1 0.4513] PawnSensing function where if the enemy AI sees the player, they then begin to start chasing after them before stopping if they lose sight of the player character.
  (Utilities|FlowControl|Sequence
    (:then_0
      (AI|AIMoveTo self "0, 0, 0" Pawn 5.0 false))
    (:then_1
      (Utilities|FlowControl|RetriggerableDelay 1.0)
      (CallFunction|TestAIRoam))))

(event OnComponentBeginOverlap(CollisionBox)
  (params (OverlappedComponent :type Primitive%20Component%20Object%20Reference) (OtherActor :type Actor%20Object%20Reference) (OtherComp :type Primitive%20Component%20Object%20Reference) (OtherBodyIndex :type Integer) (bFromSweep :type Boolean) (SweepResult :type Hit%20Result%20Structure%20%28by%20ref%29))
  (bind _returnvalue (Transformation|GetActorLocation))
  ;[0.1557 1 0.4513] Attack functionality where if the player is collding in front of the enemy AI, then they subsequently lose health based on the PlayerDamage variable.
  (bind (_outhit _returnvalue_2) (Collision|SphereTraceForObjects _returnvalue (+ _returnvalue (* (Math|Vector|GetForwardVector (Transformation|GetActorRotation)) 2.5e+02)) 1.2e+02 (Utilities|Array|MakeArray "ObjectTypeQuery3") false 0 "ForDuration"))
  (if _returnvalue_2
    (bind _asbp_first_person_character (Utilities|Casting|CastToBP_FirstPersonCharacter (.HitActor (Collision|BreakHitResult _outhit))))
    (Default|TakeDamage _asbp_first_person_character (Variables|Default|GetPlayerDamage))
    (Utilities|FlowControl|Delay 0.8)))

(event Custom|Test_AI_Roam
  ;[0.1557 1 0.4513] Function used to move second AI around the scene, without the use of a behaviour tree. This should apply to strictly static enemies.
  (AI|AIMoveTo self (.RandomLocation (AI|Navigation|GetRandomReachablePointinRadius (Transformation|GetActorLocation) 1.5e+03 0 0)) 0 5.0 false
    (:OnSuccess
      (CallFunction|TestAIRoam))))

(event EventBeginPlay
  ;[0.1557 1 0.4513] Function used to move second AI around the scene, without the use of a behaviour tree. This should apply to strictly static enemies.
  (CallFunction|TestAIRoam))

(fn ConstructionScript)