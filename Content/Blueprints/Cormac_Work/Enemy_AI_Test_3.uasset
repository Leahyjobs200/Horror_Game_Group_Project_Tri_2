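; Test horror enemy AI that turns to stare at a nearby player and chases them once spotted.
; PawnSensing starts a chase after three seconds, while a retriggerable delay calls the roam event once sightings lapse.
; Roaming re-issues AIMoveTo on success, with no destination set.
; Overlapping the presence collision starts a looping timer that eases actor yaw toward the character until overlap ends.
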(event OnSeePawn(PawnSensing)
  (params (Pawn :type Pawn%20Object%20Reference))
  ;[0.1557 1 0.4513] Test function where if the enemy AI sees the player, they then begin to start chasing after them before stopping if they lose sight of the player character. There is a delay of three seconds to allow for the hands to rotate and stare at the player, as askin to horror tropes.
  (Utilities|FlowControl|Sequence
    (:then_0
      (Utilities|FlowControl|Delay 3.0)
      (AI|AIMoveTo self "0, 0, 0" Pawn 5.0 false))
    (:then_1
      (Utilities|FlowControl|RetriggerableDelay 1.0)
      (CallFunction|TestAIRoam))))

(event OnComponentBeginOverlap(PlayerPresenceCollision)
  (params (OverlappedComponent :type Primitive%20Component%20Object%20Reference) (OtherActor :type Actor%20Object%20Reference) (OtherComp :type Primitive%20Component%20Object%20Reference) (OtherBodyIndex :type Integer) (bFromSweep :type Boolean) (SweepResult :type Hit%20Result%20Structure%20%28by%20ref%29))
  ;[0.1557 1 0.4513] If the player enters the sphere detection collision, the arms rotate to face the player. They only stop if the player exits the AI's visible range/exit the sphere collider.
  (bind _ascharacter (Utilities|Casting|CastToCharacter OtherActor))
  (Variables|Default|SetChar%20REF _ascharacter)
  (bind _returnvalue (Utilities|Time|SetTimerbyEvent (delegate Custom|Rotate) 0.01 true))
  (Variables|Default|SetTimer%20Handle _returnvalue))

(event OnComponentEndOverlap(PlayerPresenceCollision)
  (params (OverlappedComponent :type Primitive%20Component%20Object%20Reference) (OtherActor :type Actor%20Object%20Reference) (OtherComp :type Primitive%20Component%20Object%20Reference) (OtherBodyIndex :type Integer))
  ;[0.1557 1 0.4513] Contains the functionality to stop rotating after the player exits the presence zone.
  (Utilities|Time|ClearandInvalidateTimerbyHandle (Variables|Default|GetTimer%20Handle)))

(event Custom|Test_AI_Roam
  ;[0.1557 1 0.4513] Test function used to make the enemy AI move after the player, only after they have been spotted.
  (AI|AIMoveTo self "0, 0, 0" 0 5.0 false
    (:OnSuccess
      (CallFunction|TestAIRoam))))

(event Custom|Rotate
  ;[0.1557 1 0.4513] If the player enters the sphere detection collision, the arms rotate to face the player. They only stop if the player exits the AI's visible range/exit the sphere collider.
  (Transformation|SetActorRotation (Math|Rotator|MakeRotator 0.0 0.0 (.yaw (Math|Interpolation|RInterpTo (Transformation|GetActorRotation) (Math|Rotator|FindLookatRotation (Transformation|GetActorLocation) (Transformation|GetActorLocation (Variables|Default|GetChar%20REF))) (Utilities|Time|GetWorldDeltaSeconds) 1.0)))))

(event EventBeginPlay
  ;[0.1557 1 0.4513] Test function used to make the enemy AI move after the player, only after they have been spotted.
  (CallFunction|TestAIRoam))

(fn ConstructionScript)