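; Slime hand enemy that turns to face the player and summons an Enemy_SlimeMonster at the player's EnemySpawn point.
; Entering the presence collision starts a fast looping timer that smoothly interpolates yaw toward the player, and leaving clears it.
; Each rotation tick also triggers the spawn path, where a delay and DoOnce yield a single spawn with no line-of-sight check, even if the player has left.
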(event OnComponentBeginOverlap(PlayerPresenceCollision)
  (params (OverlappedComponent :type Primitive%20Component%20Object%20Reference) (OtherActor :type Actor%20Object%20Reference) (OtherComp :type Primitive%20Component%20Object%20Reference) (OtherBodyIndex :type Integer) (bFromSweep :type Boolean) (SweepResult :type Hit%20Result%20Structure%20%28by%20ref%29))
  ;[0.1557 1 0.4513] If the player enters the sphere detection collision, the slime hand rotates to face the player. They only stop if the player exits the AI's visible range/exit the sphere collider. If spotted, a slime monster will spawn behind the player.
  (bind _asbp_first_person_character (Utilities|Casting|CastToBP_FirstPersonCharacter OtherActor))
  (Variables|Default|SetChar%20REF _asbp_first_person_character)
  (bind _returnvalue (Utilities|Time|SetTimerbyEvent (delegate Custom|Rotate) 0.01 true))
  (Variables|Default|SetTimer%20Handle _returnvalue))

(event OnComponentEndOverlap(PlayerPresenceCollision)
  (params (OverlappedComponent :type Primitive%20Component%20Object%20Reference) (OtherActor :type Actor%20Object%20Reference) (OtherComp :type Primitive%20Component%20Object%20Reference) (OtherBodyIndex :type Integer))
  ;[0.1557 1 0.4513] Contains the functionality to stop rotating after the player exits the presence zone.
  (Utilities|Time|ClearandInvalidateTimerbyHandle (Variables|Default|GetTimer%20Handle)))

(event Custom|When%20Player%20Seen
  ;[0.2637 0.1604 1] If the slime hand has spotted the player, the slime monster will spawn from behind them and will subsequently then begin to chase them around.
  (bind _asbp_first_person_character (Utilities|Casting|CastToBP_FirstPersonCharacter (Game|GetPlayerCharacter 0)))
  (Utilities|FlowControl|Delay 5.0)
  (Utilities|FlowControl|DoOnce false
    (:Completed
      (Game|SpawnActorfromClass "/Game/Blueprints/Cormac_Work/Enemy_SlimeMonster.Enemy_SlimeMonster_C" (Math|Transform|MakeTransform (Transformation|GetWorldLocation (Variables|/Game/FirstPerson/Blueprints/BP_FirstPersonCharacter.BP_FirstPersonCharacter_C|GetEnemySpawn _asbp_first_person_character)) (Transformation|GetActorRotation _asbp_first_person_character)) "AdjustIfPossibleButAlwaysSpawn" "MultiplyWithRoot" 0 0))))

(event Custom|Rotate
  ;[0.1557 1 0.4513] If the player enters the sphere detection collision, the slime hand rotates to face the player. They only stop if the player exits the AI's visible range/exit the sphere collider. If spotted, a slime monster will spawn behind the player.
  (Transformation|SetActorRotation (Math|Rotator|MakeRotator 0.0 0.0 (.yaw (Math|Interpolation|RInterpTo (Transformation|GetActorRotation) (Math|Rotator|FindLookatRotation (Transformation|GetActorLocation) (Transformation|GetActorLocation (Variables|Default|GetChar%20REF))) (Utilities|Time|GetWorldDeltaSeconds) 1.0))))
  (CallFunction|WhenPlayerSeen))

(fn ConstructionScript)