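; Enemy AI controller that drives roaming and chase behaviour through the BT_EnemyAIController behaviour tree, started on BeginPlay.
; AI perception updates feed the blackboard: a successful sight stimulus stores the sensed actor as TargetActor, with no check that it is the player.
; Losing sight, or any update from a non-sight sense, clears TargetActor.
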(event OnTargetPerceptionUpdated(AIPerception)
  (params (Actor :type Actor%20Object%20Reference) (Stimulus :type AI%20Stimulus%20Structure))
  ;[1 0.01714 0.9412] Upon seeing the player in its sight, a bool value is toggled on the behaviour tree and the AI chases after the player before they lose them and the process begins again each time they are spotted.
  (bind _returnvalue (Class|AIPerceptionSystem|GetSenseClassforStimulus Stimulus))
  (if (== _returnvalue "/Script/AIModule.AISense_Sight")
    (if (.bSuccessfullySensed (Utilities|Struct|BreakAIStimulus Stimulus))
      (AI|Components|Blackboard|SetValueasObject (AI|GetBlackboard 0) (Utilities|Name|MakeLiteralName "TargetActor") Actor)
      (else
        (AI|Components|Blackboard|SetValueasObject (AI|GetBlackboard 0) (Utilities|Name|MakeLiteralName "TargetActor") 0 :!label _label)))
    (else
      (goto _label))))

(event EventBeginPlay
  ;[1 0.01714 0.9412] Calls behaviour tree to run enemy roaming AI behaviour.
  (AI|RunBehaviorTree "/Game/Blueprints/Cormac_Work/AI_Configuration/BT_EnemyAIController.BT_EnemyAIController"))

(fn ConstructionScript)