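; Door actor that teleports the player to a linked door when an actor overlap begins.
; The overlap event fades the camera and audio out over a second, then moves the player character to the ConnectedDoor's location.
; It then sets the control rotation from this door's own Arrow component and stops the camera fade.
; The overlap trigger is marked to be replaced by a custom event.
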(event Collision|EventActorBeginOverlap
  (params (OtherActor :type Actor%20Object%20Reference))
  (bind _returnvalue (Game|GetPlayerCameraManager 0))
  (CameraFades|StartCameraFade :self _returnvalue :ToAlpha 1.0 :Duration 1.0 :bShouldFadeAudio true :bHoldWhenFinished true) ; Camera fades in
  ;[1 1 1] Teleport Player
  (Utilities|FlowControl|Delay 1.0)
  (Transformation|Teleport (Game|GetPlayerCharacter 0) (Transformation|GetActorLocation (Variables|Default|GetConnectedDoor)) "0.000000,0.000000,0.000000")
  ;[1 1 1] Set player rotation
  (Pawn|SetControlRotation (Game|GetPlayerController 0) (Transformation|GetWorldRotation (Variables|Default|GetArrow)))
  (CameraFades|StopCameraFade _returnvalue) ; Camera fades out
)

(fn ConstructionScript)