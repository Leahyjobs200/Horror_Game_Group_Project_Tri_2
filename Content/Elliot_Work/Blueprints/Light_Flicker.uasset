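; Light flicker actor that randomly blinks a rect light off and back on.
; Tick feeds a Delay of a random whole number of seconds from 0 to 9, then hides the light and restores it after one second.
; The latent Delays ignore re-triggers while pending, so calling them every frame produces a repeating irregular cycle.
; A play-sound call at the light's location is present but unconnected, so it never runs.
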(event EventBeginPlay)

(event Collision|EventActorBeginOverlap
  (params (OtherActor :type Actor%20Object%20Reference)))

(event EventTick
  (params (DeltaSeconds :type Float%20%28single-precision%29))
  (Utilities|FlowControl|Delay (Math|Conversions|ToFloat(Integer) (Math|Random|RandomInteger 10)))
  (Rendering|SetVisibility (Variables|Default|GetRectLight) false false)
  (Utilities|FlowControl|Delay 1.0)
  (Rendering|SetVisibility (Variables|Default|GetRectLight) true false))

(fn ConstructionScript)