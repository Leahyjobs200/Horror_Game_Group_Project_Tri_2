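; Room-exit controller that unlocks the way out once the player has checked both the leaflet and the TV.
; On BeginPlay it reads both flags from the game instance's save data, then runs ReplaceDoor.
; When both are true, ReplaceDoor swaps the fake and real doors by moving them vertically.
; If the objective increment actor is at 1, it shows a delayed, one-time checkout thought and front-desk bell objective.
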(event Custom|ReplaceDoor
  (if (and (Variables|Default|GetCheckedLeaflet?) (Variables|Default|GetCheckedTV?))
    (Transformation|SetActorLocation (Variables|Default|GetFakeDoor) "-4655.510630,1375.803368,-131.093757" false false)
    (Transformation|SetActorLocation (Variables|Default|GetRealDoor) "-4655.510630,1375.803368,131.093757" false false)
    (bind _outactors (Actor|GetAllActorsOfClass "/Game/Elliot_Work_2/Blueprints/BP_ObjectiveIncrement.BP_ObjectiveIncrement_C"))
    (if (== (Variables|/Game/Elliot_Work_2/Blueprints/BP_ObjectiveIncrement.BP_ObjectiveIncrement_C|GetIncrement (Utilities|Array|Get(acopy) _outactors)) 1)
      (Utilities|FlowControl|DoOnce false
        (:Completed
          (Utilities|FlowControl|Delay 1.9)
          (bind _asbp_first_person_character (Utilities|Casting|CastToBP_FirstPersonCharacter (Game|GetPlayerCharacter 0)))
          (Default|UpdateThoughts _asbp_first_person_character "About time I checked out at the front desk and headed home, last night felt like a fever dream!")
          (Default|UpdateObjective _asbp_first_person_character "Ring bell at front desk")
          (bind _newparam (Default|GetPlayerUI _asbp_first_person_character))
          (UserInterface|Animation|PlayAnimation _newparam (Variables|/Game/Elliot_Work_2/HUD/Player_UI.Player_UI_C|GetThoughts_fade _newparam) 0.0 1 "Forward" 1.0 false))))))

(event EventBeginPlay
  (bind _returnvalue (Game|GetGameInstance))
  (bind _asgi_basic_game_instance (Utilities|Casting|CastToGI_BasicGameInstance _returnvalue))
  (bind _savedata (Variables|/Game/Elliot_Work_2/Blueprints/Game_Instance/GI_BasicGameInstance.GI_BasicGameInstance_C|GetSaveData _asgi_basic_game_instance))
  (bind (_charstats _lastlevelsavedat _savedtransform _loopincrement _objectiveincrement _checkedleafletatstart _checkedtvatstart) (Utilities|Struct|BreakS_SaveData _savedata))
  (Variables|Default|SetCheckedLeaflet? _checkedleafletatstart)
  (Variables|Default|SetCheckedTV? _checkedtvatstart)
  (CallFunction|ReplaceDoor))

(fn ConstructionScript)