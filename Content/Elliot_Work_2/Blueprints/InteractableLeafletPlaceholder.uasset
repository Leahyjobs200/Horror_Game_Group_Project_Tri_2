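; An interactable placeholder leaflet actor that shows a leaflet widget and updates the player's respawn location.
; On BeginPlay it creates the Leaflet_Placeholder widget and stores it.
; When Interact fires and the widget is not on screen, it adds it to the viewport and copies the indexed entry from RespawnPoint's RespawnPoints array into the first-person character's RespawnLocation.
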(event EventBeginPlay
  (bind _returnvalue (UserInterface|CreateWidget "/Game/Elliot_Work_2/HUD/Leaflet_Placeholder.Leaflet_Placeholder_C"))
  (Variables|Default|SetLeaflet _returnvalue))

(event Collision|EventActorBeginOverlap
  (params (OtherActor :type Actor%20Object%20Reference)))

(event EventTick
  (params (DeltaSeconds :type Float%20%28single-precision%29)))

(event EventInteract
  (bind _leaflet (Variables|Default|GetLeaflet))
  (if (not (UserInterface|Viewport|IsinViewport _leaflet))
    (UserInterface|Viewport|AddtoViewport _leaflet 0)
    (Variables|/Game/FirstPerson/Blueprints/BP_FirstPersonCharacter.BP_FirstPersonCharacter_C|SetRespawnLocation (.AsBP%20First%20Person%20Character (Utilities|Casting|CastToBP_FirstPersonCharacter (Game|GetPlayerCharacter 0))) (Utilities|Array|Get(acopy) (Variables|/Game/Elliot_Work_2/Blueprints/RespawnPoint.RespawnPoint_C|GetRespawnPoints (Variables|Default|GetRespawnPoint)) (Variables|Default|GetIndex)))))

(fn ConstructionScript)