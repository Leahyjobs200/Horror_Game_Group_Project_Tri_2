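; FinalObjectiveTrigger is a one-shot overlap box that gives the player the objective of finding fuse boxes until escape, with an explanatory thought.
; On first overlap it calls TriggerObjective on the first BP_ObjectiveIncrement found in the level.
; After a short delay it pushes a follow-up thought through BP_FirstPersonCharacter and plays the player UI's ThoughtsFade animation.
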(event OnComponentBeginOverlap(Box)
  (params (OverlappedComponent :type Primitive%20Component%20Object%20Reference) (OtherActor :type Actor%20Object%20Reference) (OtherComp :type Primitive%20Component%20Object%20Reference) (OtherBodyIndex :type Integer) (bFromSweep :type Boolean) (SweepResult :type Hit%20Result%20Structure%20%28by%20ref%29))
  (bind _returnvalue (Game|GetPlayerCharacter 0))
  (bind _asbp_first_person_character (Utilities|Casting|CastToBP_FirstPersonCharacter _returnvalue))
  (Utilities|FlowControl|DoOnce false
    (:Completed
      (bind _outactors (Actor|GetAllActorsOfClass "/Game/Elliot_Work_2/Blueprints/BP_ObjectiveIncrement.BP_ObjectiveIncrement_C"))
      (Default|TriggerObjective (Utilities|Array|Get(acopy) _outactors) 13 "Find other fuse boxes until escaped" "So, the goal is to loop around the corridors. Find odd changes in 
the halls and locate the fuse boxes to activate the power!" 0 false)
      (Utilities|FlowControl|Delay 5.0)
      (Default|UpdateThoughts _asbp_first_person_character "If I find all of them I can escape this place!")
      (bind _newparam (Default|GetPlayerUI _asbp_first_person_character))
      (UserInterface|Animation|PlayAnimation _newparam (Variables|/Game/Elliot_Work_2/HUD/Player_UI.Player_UI_C|GetThoughts_fade _newparam) 0.0 1 "Forward" 1.0 false))))

(fn ConstructionScript)