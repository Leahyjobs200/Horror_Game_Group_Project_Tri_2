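; A trigger volume, LiftReactionTrigger, that shows the player character's reaction as a thought on screen.
; When the player overlaps it, it finds the LoopIncrement actor and continues only if the loop stage is at least one.
; A DoOnce then updates the first-person character's thoughts and plays the ThoughtsFade animation on the player UI, so the reaction fires a single time.
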(event OnComponentBeginOverlap(Trigger)
  (params (OverlappedComponent :type Primitive%20Component%20Object%20Reference) (OtherActor :type Actor%20Object%20Reference) (OtherComp :type Primitive%20Component%20Object%20Reference) (OtherBodyIndex :type Integer) (bFromSweep :type Boolean) (SweepResult :type Hit%20Result%20Structure%20%28by%20ref%29))
  (bind _returnvalue (Game|GetPlayerCharacter 0))
  (if (or (== OtherActor _returnvalue) (== OtherActor (.AsBP%20First%20Person%20Character (Utilities|Casting|CastToBP_FirstPersonCharacter _returnvalue))))
    (bind _outactors (Actor|GetAllActorsOfClass "/Game/Blueprints/David_Work/Blueprints_and_Actors/LoopIncrement.LoopIncrement_C"))
    (if (>= (Variables|/Game/Blueprints/David_Work/Blueprints_and_Actors/LoopIncrement.LoopIncrement_C|GetLoopStage (Utilities|Array|Get(acopy) _outactors)) 1)
      (Utilities|FlowControl|DoOnce false
        (:Completed
          (bind _asbp_first_person_character (Utilities|Casting|CastToBP_FirstPersonCharacter (Game|GetPlayerCharacter 0)))
          (Default|UpdateThoughts _asbp_first_person_character (Variables|Default|GetNewThoughtsToSet))
          (bind _newparam (Default|GetPlayerUI _asbp_first_person_character))
          (UserInterface|Animation|PlayAnimation _newparam (Variables|/Game/Elliot_Work_2/HUD/Player_UI.Player_UI_C|GetThoughts_fade _newparam) 0.0 1 "Forward" 1.0 false))))))

(fn ConstructionScript)