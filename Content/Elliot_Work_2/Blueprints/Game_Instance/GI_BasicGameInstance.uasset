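; Game instance that manages menu widgets and save slots: new game, load, delete and save.
; Menu events recreate their widgets, while LoadGame records the active slot, creates a loading screen and opens the saved level or FirstPersonMap.
; Save writes level name, player transform, stats and progress into that slot, reading world state from the first actor found of several controller and puzzle classes.
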(event Custom|RemoveLoadingScreen
  ;[1 1 1] Loading Screen
  (bind _myloadingscreen (Variables|Default|GetMyLoadingScreen)
    (:then
      (Widget|RemovefromParent _myloadingscreen))
    (:else)))

(event Custom|CreateLoadingScreen
  ;[1 1 1] Loading Screen
  (bind _myloadingscreen (Variables|Default|GetMyLoadingScreen)
    (:then
      (Widget|RemovefromParent _myloadingscreen))
    (:else
      _))
  (bind _returnvalue (UserInterface|CreateWidget "/Game/Elliot_Work_2/HUD/LoadingScreen.LoadingScreen_C" (Game|GetPlayerController 0)))
  (Variables|Default|SetMyLoadingScreen _returnvalue))

(event Custom|ShowMainMenu
  ;[1 1 1] Main Screen Commands
  (bind _mymainmenu (Variables|Default|GetMyMainMenu)
    (:then
      (Widget|RemovefromParent _mymainmenu))
    (:else
      _))
  (bind _returnvalue (UserInterface|CreateWidget "/Game/Elliot_Work_2/HUD/MainMenu.MainMenu_C" (Game|GetPlayerController 0)))
  (bind _output_get (Variables|Default|SetMyMainMenu _returnvalue))
  (UserInterface|Viewport|AddtoViewport _output_get 0))

(event Custom|NewGame
  (params (Game%20Slot :type String))
  ;[1 1 1] Main Screen Commands
  (bind _mynewgamewindow (Variables|Default|GetMyNewGameWindow)
    (:then
      (Widget|RemovefromParent _mynewgamewindow))
    (:else
      _))
  (bind _returnvalue (UserInterface|CreateWidget "/Game/Elliot_Work_2/HUD/NewGameWidget.NewGameWidget_C" (Game|GetPlayerController 0) Game%20Slot))
  (bind _output_get (Variables|Default|SetMyNewGameWindow _returnvalue))
  (UserInterface|Viewport|AddtoViewport _output_get 0))

(event Custom|LoadGame
  (params (Save%20Game%20to%20Load :type String))
  (bind _returnvalue (Game|GetPlayerController 0))
  ;[1 1 1] Main Screen Commands
  (Variables|Default|SetMyCurrentSaveSlot Save%20Game%20to%20Load)
  (bind _returnvalue_2 (SaveGame|DoesSaveGameExist Save%20Game%20to%20Load))
  (if _returnvalue_2
    (bind _returnvalue_3 (SaveGame|LoadGamefromSlot Save%20Game%20to%20Load))
    (bind _assg_my_save_game (Utilities|Casting|CastToSG_MySaveGame _returnvalue_3))
    (CallFunction|CreateLoadingScreen)
    (Variables|Default|SetSaveData (Variables|/Game/Elliot_Work_2/Blueprints/Game_Instance/SaveGame/SG_MySaveGame.SG_MySaveGame_C|GetMySaveData _assg_my_save_game))
    (if (Utilities|Enum|NotEqual(Enum) (.LastLevelSavedAt (Utilities|Struct|BreakS_SaveData (Variables|Default|GetSaveData))) "")
      (Game|OpenLevel(byName) (Utilities|String|StringToName (.LastLevelSavedAt (Utilities|Struct|BreakS_SaveData (Variables|Default|GetSaveData)))))
      (else
        (Game|OpenLevel(byName) "FirstPersonMap")))
    (Input|SetInputModeGameOnly _returnvalue false)
    (Variables|/Script/Engine.PlayerController|SetbShowMouseCursor _returnvalue false)
    (else
      (Development|PrintString (Utilities|String|ToString(Text) (Utilities|Text|FormatText "Failed to load save {save}" Save%20Game%20to%20Load))))))

(event Custom|DeleteGame
  (params (Target%20Save%20Game :type String))
  ;[1 1 1] Main Screen Commands
  (bind _returnvalue (SaveGame|DoesSaveGameExist Target%20Save%20Game))
  (if _returnvalue
    (SaveGame|DeleteGameinSlot Target%20Save%20Game)))

(event Custom|ShowSaveSelect
  ;[1 1 1] Main Screen Commands
  (bind _mysaveselect (Variables|Default|GetMySaveSelect)
    (:then
      (Widget|RemovefromParent _mysaveselect))
    (:else
      _))
  (bind _returnvalue (UserInterface|CreateWidget "/Game/Elliot_Work_2/HUD/SaveSelect.SaveSelect_C" (Game|GetPlayerController 0)))
  (bind _output_get (Variables|Default|SetMySaveSelect _returnvalue))
  (UserInterface|Viewport|AddtoViewport _output_get 0))

(event Custom|Save
  (bind _returnvalue (Game|GetPlayerCharacter 0))
  (bind _asbp_first_person_character (Utilities|Casting|CastToBP_FirstPersonCharacter _returnvalue))
  ;[1 1 1] Save variables
  (bind _returnvalue_2 (SaveGame|LoadGamefromSlot (Variables|Default|GetMyCurrentSaveSlot)))
  (bind _returnvalue_3 (Game|GetCurrentLevelName true))
  (bind _outactors (Actor|GetAllActorsOfClass "/Game/Blueprints/David_Work/Blueprints_and_Actors/Lobby_Changer.Lobby_Changer_C"))
  (bind _outactors_2 (Actor|GetAllActorsOfClass "/Game/Elliot_Work_2/Blueprints/BP_ObjectiveIncrement.BP_ObjectiveIncrement_C"))
  (bind _outactors_3 (Actor|GetAllActorsOfClass "/Game/Elliot_Work_2/Blueprints/LeaveRoomController.LeaveRoomController_C"))
  (bind _outactors_4 (Actor|GetAllActorsOfClass "/Game/Elliot_Work_2/Blueprints/LightsController.LightsController_C"))
  (bind _outactors_5 (Actor|GetAllActorsOfClass "/Game/Blueprints/David_Work/Blueprints_and_Actors/JanitorRoom/MannequinDummy.MannequinDummy_C"))
  (Utilities|Struct|SetmembersinS_SaveData (Variables|/Game/Elliot_Work_2/Blueprints/Game_Instance/SaveGame/SG_MySaveGame.SG_MySaveGame_C|GetMySaveData (.AsSG%20My%20Save%20Game (Utilities|Casting|CastToSG_MySaveGame _returnvalue_2))) _returnvalue_3 (Transformation|GetActorTransform _asbp_first_person_character) (Variables|/Game/Blueprints/David_Work/Blueprints_and_Actors/LoopIncrement.LoopIncrement_C|GetLoopStage (Variables|/Game/Blueprints/David_Work/Blueprints_and_Actors/Lobby_Changer.Lobby_Changer_C|GetLoopRef (Utilities|Array|Get(acopy) _outactors))) (Variables|/Game/Elliot_Work_2/Blueprints/BP_ObjectiveIncrement.BP_ObjectiveIncrement_C|GetIncrement (Utilities|Array|Get(acopy) _outactors_2)) (Variables|/Game/Elliot_Work_2/Blueprints/LeaveRoomController.LeaveRoomController_C|GetCheckedLeaflet? (Utilities|Array|Get(acopy) _outactors_3)) (Variables|/Game/Elliot_Work_2/Blueprints/LeaveRoomController.LeaveRoomController_C|GetCheckedTV? (Utilities|Array|Get(acopy) _outactors_3)) (Variables|/Game/FirstPerson/Blueprints/BP_FirstPersonCharacter.BP_FirstPersonCharacter_C|GetHasKeycard _asbp_first_person_character) (Variables|/Game/Elliot_Work_2/Blueprints/LightsController.LightsController_C|GetLobby%20Low (Utilities|Array|Get(acopy) _outactors_4)) (Variables|/Game/Elliot_Work_2/Blueprints/LightsController.LightsController_C|GetLobby%20Off (Utilities|Array|Get(acopy) _outactors_4)) (Variables|/Game/Elliot_Work_2/Blueprints/LightsController.LightsController_C|GetLobby%20On (Utilities|Array|Get(acopy) _outactors_4)) (Variables|/Game/Blueprints/David_Work/Blueprints_and_Actors/JanitorRoom/MannequinDummy.MannequinDummy_C|GetMannequinStage (Utilities|Array|Get(acopy) _outactors_5)))
  (bind _objective (Default|GetObjective _asbp_first_person_character))
  (bind _thoughts (Default|GetThoughts _asbp_first_person_character))
  (Utilities|Struct|SetmembersinS_CharStats (Utilities|Struct|BreakS_SaveData (Variables|/Game/Elliot_Work_2/Blueprints/Game_Instance/SaveGame/SG_MySaveGame.SG_MySaveGame_C|GetMySaveData (.AsSG%20My%20Save%20Game (Utilities|Casting|CastToSG_MySaveGame _returnvalue_2)))) (Variables|/Game/Elliot_Work_2/Blueprints/Player_Components/PlayerHealth_Component.PlayerHealth_Component_C|GetCurrentHealth (Variables|/Game/FirstPerson/Blueprints/BP_FirstPersonCharacter.BP_FirstPersonCharacter_C|GetPlayerHealth_Component _asbp_first_person_character)) (Variables|/Game/Elliot_Work_2/Blueprints/Player_Components/PlayerStamina_Component.PlayerStamina_Component_C|GetCurrentStamina (Variables|/Game/FirstPerson/Blueprints/BP_FirstPersonCharacter.BP_FirstPersonCharacter_C|GetPlayerStamina_Component _asbp_first_person_character)) _objective _thoughts)
  (SaveGame|SaveGametoSlot (.AsSG%20My%20Save%20Game (Utilities|Casting|CastToSG_MySaveGame _returnvalue_2)) (Variables|Default|GetMyCurrentSaveSlot)))