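; Placeholder TV actor that the player can interact with to toggle its cube's look and advance the leave-room sequence.
; Interact runs a FlipFlop that alternates the cube between a basic shape material and black.
; The first toggle also updates the character's thoughts with a UI fade animation, then marks CheckedTV on the first LeaveRoomController found and calls its ReplaceDoor.
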(event EventBeginPlay)

(event Collision|EventActorBeginOverlap
  (params (OtherActor :type Actor%20Object%20Reference)))

(event EventTick
  (params (DeltaSeconds :type Float%20%28single-precision%29)))

(event EventInteract
  (bind _cube (Variables|Default|GetCube))
  (Utilities|FlowControl|FlipFlop
    (:A
      (Rendering|Material|SetMaterial _cube 0 "/Engine/BasicShapes/BasicShapeMaterial.BasicShapeMaterial")
      (Utilities|FlowControl|DoOnce false
        (:Completed
          (bind _asbp_first_person_character (Utilities|Casting|CastToBP_FirstPersonCharacter (Game|GetPlayerCharacter 0)))
          (Default|UpdateThoughts _asbp_first_person_character (Variables|Default|GetNewThoughtsToSet))
          (bind _newparam (Default|GetPlayerUI _asbp_first_person_character))
          (UserInterface|Animation|PlayAnimation _newparam (Variables|/Game/Elliot_Work_2/HUD/Player_UI.Player_UI_C|GetThoughts_fade _newparam) 0.0 1 "Forward" 1.0 false)
          (bind _outactors (Actor|GetAllActorsOfClass "/Game/Elliot_Work_2/Blueprints/LeaveRoomController.LeaveRoomController_C"))
          (Variables|/Game/Elliot_Work_2/Blueprints/LeaveRoomController.LeaveRoomController_C|SetCheckedTV? (Utilities|Array|Get(acopy) _outactors) true)
          (Default|ReplaceDoor (Utilities|Array|Get(acopy) _outactors)))))
    (:B
      (Rendering|Material|SetMaterial _cube 0 "/Game/Elliot_Work_2/Materials/M_Black.M_Black"))))

(fn ConstructionScript)