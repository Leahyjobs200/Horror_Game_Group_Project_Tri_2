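; Trigger actor that swaps a fake door and a real door, apparently for the janitor door.
; The first actor overlap, gated by a DoOnce, moves FakeDoor into the doorway position and lifts RealDoor far above it.
; MoveDoorBack reverses the swap, but nothing in this Blueprint calls it.
; Both doors teleport between hardcoded world locations without sweeping.
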(event Custom|MoveDoor
  (Transformation|SetActorLocation (Variables|Default|GetFakeDoor) "-2047.000000,2334.000000,135.000000" false false)
  (Transformation|SetActorLocation (Variables|Default|GetRealDoor) "-2047.000000,2334.000000,1300.000000" false false))

(event Custom|MoveDoorBack
  (Transformation|SetActorLocation (Variables|Default|GetRealDoor) "-2047.000000,2334.000000,135.000000" false false)
  (Transformation|SetActorLocation (Variables|Default|GetFakeDoor) "-2047.000000,2334.000000,1300.000000" false false))

(event Collision|EventActorBeginOverlap
  (params (OtherActor :type Actor%20Object%20Reference))
  (Utilities|FlowControl|DoOnce false
    (:Completed
      (CallFunction|MoveDoor))))

(fn ConstructionScript)