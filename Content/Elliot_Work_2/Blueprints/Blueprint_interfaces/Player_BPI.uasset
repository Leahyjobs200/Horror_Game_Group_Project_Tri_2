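; Player_BPI is a Blueprint Interface that declares the functions for querying and changing player state.
; It covers taking damage, adding and reading health, reading stamina, and getting objective and thoughts text.
; Torch functions report whether a torch is held and lit, set both states, and declare a getter for the torch component.
; It holds only signatures, leaving the logic to implementing classes.
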(fn TakeDamage
  (params (Amount :type Float%20%28double-precision%29)))

(fn AddHealth
  (params (Amount :type Float%20%28double-precision%29)))

(fn GetHealth
  (return 0.0 0.0))

(fn GetStamina
  (return 0.0 0.0))

(fn GetObjective
  (return ""))

(fn GetThoughts
  (return ""))

(fn TorchOn?
  (return false false))

(fn GetTorchComponent
  (return 0))

(fn SetTorch
  (params (HasTorch? :type Boolean) (TorchOn? :type Boolean)))