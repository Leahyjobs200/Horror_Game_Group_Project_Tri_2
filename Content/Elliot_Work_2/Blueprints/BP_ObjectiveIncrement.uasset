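; BP_ObjectiveIncrement tracks objective progression with a counter so that objectives trigger in sequence.
; TriggerObjective acts only when the supplied index matches the counter, then passes the new objective and thoughts to the first-person character and plays the UI's thoughts fade animation.
; It then advances the counter and can optionally set the character's respawn location to the matching entry in the supplied respawn point list.
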(fn ConstructionScript)

(fn Increment+
  (Math|Integer|IncrementInt (Variables|Default|GetIncrement)))

(fn TriggerObjective
  (params (Index :type Integer) (NewObjectiveToSet :type String) (NewThroughtsToSet :type String) (RespawnPoint :type Respawn%20Point%20Object%20Reference) (UpdateRespawn? :type Boolean))
  (if (== (Variables|Default|GetIncrement) Index)
    (bind _asbp_first_person_character (Utilities|Casting|CastToBP_FirstPersonCharacter (Game|GetPlayerCharacter 0)))
    (Utilities|FlowControl|DoOnce false
      (:Completed
        (Default|UpdateObjective _asbp_first_person_character NewObjectiveToSet)
        (Default|UpdateThoughts _asbp_first_person_character NewThroughtsToSet)
        (bind _newparam (Default|GetPlayerUI _asbp_first_person_character))
        (UserInterface|Animation|PlayAnimation _newparam (Variables|/Game/Elliot_Work_2/HUD/Player_UI.Player_UI_C|GetThoughts_fade _newparam) 0.0 1 "Forward" 1.0 false)
        (CallFunction|Increment+)
        (if UpdateRespawn?
          (Variables|/Game/FirstPerson/Blueprints/BP_FirstPersonCharacter.BP_FirstPersonCharacter_C|SetRespawnLocation (.AsBP%20First%20Person%20Character (Utilities|Casting|CastToBP_FirstPersonCharacter (Game|GetPlayerCharacter 0))) (Utilities|Array|Get(acopy) (Variables|/Game/Elliot_Work_2/Blueprints/RespawnPoint.RespawnPoint_C|GetRespawnPoints RespawnPoint) Index)))))))