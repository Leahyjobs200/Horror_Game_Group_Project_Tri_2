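; Interactable bell that plays a ring sound at its cube on every interaction and advances the player's objective after the first ring.
; A DoOnce gates the first-ring sequence: it sets a thought on the first-person character hinting to ring again and plays the UI's thought fade.
; After a delay, it calls TriggerObjective on the first BP_ObjectiveIncrement with its configured objective data and a respawn update.
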(event EventInteract
  (bind _returnvalue (Game|GetPlayerCharacter 0))
  (bind _asbp_first_person_character (Utilities|Casting|CastToBP_FirstPersonCharacter _returnvalue))
  (Audio|PlaySoundatLocation "/Game/External_Assets/Bell_SE/mixkit-bike-notification-bell-590.mixkit-bike-notification-bell-590" (Transformation|GetWorldLocation (Variables|Default|GetCube)) "0, 0, 0" 1.0 1.0 0.0 0 0 0 0)
  (Utilities|FlowControl|DoOnce false
    (:Completed
      (bind _newparam (Default|GetPlayerUI _asbp_first_person_character))
      (Default|UpdateThoughts _asbp_first_person_character "Maybe I should ring it some more.")
      (UserInterface|Animation|PlayAnimation _newparam (Variables|/Game/Elliot_Work_2/HUD/Player_UI.Player_UI_C|GetThoughts_fade _newparam) 0.0 1 "Forward" 1.0 false)
      (Utilities|FlowControl|Delay 7.5)
      (bind _outactors (Actor|GetAllActorsOfClass "/Game/Elliot_Work_2/Blueprints/BP_ObjectiveIncrement.BP_ObjectiveIncrement_C"))
      (Default|TriggerObjective (Utilities|Array|Get(acopy) _outactors) (Variables|Default|GetIndex) (Variables|Default|GetnewObjectiveToSet) (Variables|Default|GetnewThoughtsToSet) (Variables|Default|GetRespawnPoint) true))))

(fn ConstructionScript)