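; Trigger volume that advances the player's objective when they find the fuse box.
; When the player overlaps its box, it checks that the BP_ObjectiveIncrement actor is on step 12 and that LobbyChanger's loop reference has reached stage 4 or later.
; If both hold, it fires TriggerObjective once, setting a new objective to interact with the fuse box and a thought noting that looping around was the answer.
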(event OnComponentBeginOverlap(Box)
  (params (OverlappedComponent :type Primitive%20Component%20Object%20Reference) (OtherActor :type Actor%20Object%20Reference) (OtherComp :type Primitive%20Component%20Object%20Reference) (OtherBodyIndex :type Integer) (bFromSweep :type Boolean) (SweepResult :type Hit%20Result%20Structure%20%28by%20ref%29))
  (bind _returnvalue (Game|GetPlayerCharacter 0))
  (if (or (== OtherActor _returnvalue) (== OtherActor (.AsBP%20First%20Person%20Character (Utilities|Casting|CastToBP_FirstPersonCharacter _returnvalue))))
    (bind _outactors (Actor|GetAllActorsOfClass "/Game/Elliot_Work_2/Blueprints/BP_ObjectiveIncrement.BP_ObjectiveIncrement_C"))
    (if (== (Variables|/Game/Elliot_Work_2/Blueprints/BP_ObjectiveIncrement.BP_ObjectiveIncrement_C|GetIncrement (Utilities|Array|Get(acopy) _outactors)) 12)
      (if (>= (Variables|/Game/Blueprints/David_Work/Blueprints_and_Actors/LoopIncrement.LoopIncrement_C|GetLoopStage (Variables|/Game/Blueprints/David_Work/Blueprints_and_Actors/Lobby_Changer.Lobby_Changer_C|GetLoopRef (Variables|Default|GetLobbyChanger))) 4)
        (Utilities|FlowControl|DoOnce false
          (:Completed
            (bind _outactors_2 (Actor|GetAllActorsOfClass "/Game/Elliot_Work_2/Blueprints/BP_ObjectiveIncrement.BP_ObjectiveIncrement_C"))
            (Default|TriggerObjective (Utilities|Array|Get(acopy) _outactors_2) 12 "Interact with fuse box." "THE FUSE BOX! It’s there! Looping around was the answer!" 0 false)))))))

(event EventBeginPlay)

(event Collision|EventActorBeginOverlap
  (params (OtherActor :type Actor%20Object%20Reference)))

(event EventTick
  (params (DeltaSeconds :type Float%20%28single-precision%29)))

(fn ConstructionScript)