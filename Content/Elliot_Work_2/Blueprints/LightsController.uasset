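; Controller that switches the ceiling lights of the lobby and two upper-floor areas between on, low and off.
; SetLights stores per-area change and state flags, then calls ChangeLights to pick the matching event.
; Each event fakes the lighting state by swapping an emissive material on that ceiling mesh.
; The branches are chained, so once one area's state is applied, later areas are skipped in that call.
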(event Custom|SetLights
  (params (ChangeLobby :type Boolean) (LobbyOn :type Boolean) (LobbyLow :type Boolean) (LobbyOff :type Boolean) (ChangeUpper :type Boolean) (UpperOn :type Boolean) (UpperLow :type Boolean) (UpperOff :type Boolean) (ChangeUpper2 :type Boolean) (Upper2On :type Boolean) (Upper2Low :type Boolean) (Upper2Off :type Boolean))
  ;[1 1 1] Set which lights and what setting
  (Variables|Default|SetChange%20Lobby ChangeLobby)
  (Variables|Default|SetLobby%20On LobbyOn)
  (Variables|Default|SetLobby%20Low LobbyLow)
  (Variables|Default|SetLobby%20Off LobbyOff)
  (Variables|Default|SetChange%20Upper ChangeUpper)
  (Variables|Default|SetUpper%20On UpperOn)
  (Variables|Default|SetUpper%20Low UpperLow)
  (Variables|Default|SetUpper%20Off UpperOff)
  (Variables|Default|SetChange%20Upper%202 ChangeUpper2)
  (Variables|Default|SetUpper%202On Upper2On)
  (Variables|Default|SetUpper%202Low Upper2Low)
  (Variables|Default|SetUpper%202Off Upper2Off)
  (CallFunction|ChangeLights))

(event Custom|LobbyLightsLow
  ;[1 1 1] Change Material
  (Rendering|Material|SetMaterial (Variables|/Script/Engine.StaticMeshActor|GetStaticMeshComponent (Variables|Default|GetLobbyCeiling)) 1 "/Game/MaterialsMAIN/I_EmmisiveLightsLow.I_EmmisiveLightsLow"))

(event Custom|UpperFloor2LightsOff
  ;[1 1 1] Change Material
  (Rendering|Material|SetMaterial (Variables|/Script/Engine.StaticMeshActor|GetStaticMeshComponent (Variables|Default|GetUpperFloorCeiling2)) 1 "/Game/MaterialsMAIN/I_EmmisiveLightsOff.I_EmmisiveLightsOff"))

(event Custom|LobbyLightsOff
  ;[1 1 1] Change Material
  (Rendering|Material|SetMaterial (Variables|/Script/Engine.StaticMeshActor|GetStaticMeshComponent (Variables|Default|GetLobbyCeiling)) 1 "/Game/MaterialsMAIN/I_EmmisiveLightsOff.I_EmmisiveLightsOff"))

(event Custom|LobbyLightsOn
  ;[1 1 1] Change Material
  (Rendering|Material|SetMaterial (Variables|/Script/Engine.StaticMeshActor|GetStaticMeshComponent (Variables|Default|GetLobbyCeiling)) 1 "/Game/MaterialsMAIN/I_EmmisiveLights.I_EmmisiveLights"))

(event Custom|ChangeLights
  ;[1 1 1] Change Lights
  (if (Variables|Default|GetChange%20Lobby)
    (if (Variables|Default|GetLobby%20On)
      (CallFunction|LobbyLightson)
      (elif (Variables|Default|GetLobby%20Low)
        (CallFunction|LobbyLightsLow)
        (elif (Variables|Default|GetLobby%20Off)
          (CallFunction|LobbyLightsOff)
          (else
            (if (Variables|Default|GetChange%20Upper) :!label _label
              (if (Variables|Default|GetUpper%20On)
                (CallFunction|UpperFloorLightson)
                (elif (Variables|Default|GetUpper%20Low)
                  (CallFunction|UpperFloorLightsL)
                  (elif (Variables|Default|GetUpper%20Off)
                    (CallFunction|UpperFloorLightsO)
                    (else
                      (if (Variables|Default|GetChange%20Upper%202) :!label _label_2
                        (if (Variables|Default|GetUpper%202On)
                          (CallFunction|UpperFloor2Lightson)
                          (elif (Variables|Default|GetUpper%202Low)
                            (CallFunction|UpperFloor2LightsLow)
                            (elif (Variables|Default|GetUpper%202Off)
                              (CallFunction|UpperFloor2LightsOff)))))))))
              (else
                (goto _label_2)))))))
    (else
      (goto _label))))

(event Custom|UpperFloorLightsOn
  ;[1 1 1] Change Material
  (Rendering|Material|SetMaterial (Variables|/Script/Engine.StaticMeshActor|GetStaticMeshComponent (Variables|Default|GetUpperFloorCeiling)) 1 "/Game/MaterialsMAIN/I_EmmisiveLights.I_EmmisiveLights"))

(event Custom|UpperFloorLightsL
  ;[1 1 1] Change Material
  (Rendering|Material|SetMaterial (Variables|/Script/Engine.StaticMeshActor|GetStaticMeshComponent (Variables|Default|GetUpperFloorCeiling)) 1 "/Game/MaterialsMAIN/I_EmmisiveLightsLow.I_EmmisiveLightsLow"))

(event Custom|UpperFloorLightsO
  ;[1 1 1] Change Material
  (Rendering|Material|SetMaterial (Variables|/Script/Engine.StaticMeshActor|GetStaticMeshComponent (Variables|Default|GetUpperFloorCeiling)) 1 "/Game/MaterialsMAIN/I_EmmisiveLightsOff.I_EmmisiveLightsOff"))

(event Custom|UpperFloor2LightsOn
  ;[1 1 1] Change Material
  (Rendering|Material|SetMaterial (Variables|/Script/Engine.StaticMeshActor|GetStaticMeshComponent (Variables|Default|GetUpperFloorCeiling2)) 1 "/Game/MaterialsMAIN/I_EmmisiveLights.I_EmmisiveLights"))

(event Custom|UpperFloor2LightsLow
  ;[1 1 1] Change Material
  (Rendering|Material|SetMaterial (Variables|/Script/Engine.StaticMeshActor|GetStaticMeshComponent (Variables|Default|GetUpperFloorCeiling2)) 1 "/Game/MaterialsMAIN/I_EmmisiveLightsLow.I_EmmisiveLightsLow"))

(fn ConstructionScript)