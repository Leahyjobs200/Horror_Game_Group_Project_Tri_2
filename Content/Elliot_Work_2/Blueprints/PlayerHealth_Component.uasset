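; Player health component that tracks current health, starting at max, and handles damage, healing and automatic regeneration.
; ChangeHealth uses a bool to add or subtract the absolute amount, clamped between zero and max.
; While health is below max, each change sets a looping timer by function name for regeneration.
; Each regeneration tick adds a base amount and clears the timer once health is full.
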(event Custom|Regenerate%20Health
  ;[1 1 1] Regenerates health when taken
  (bind _output_get (Variables|Default|SetCurrentHealth (Math|Float|Clamp(Float) (+ (Variables|Default|GetCurrentHealth) (Variables|Default|GetBaseRegenAmount)) 0.0 (Variables|Default|GetMaxHealth))))
  ;[1 1 1] Clears the function once reached max health
  (if (>= _output_get (Variables|Default|GetMaxHealth))
    (Utilities|Time|ClearandInvalidateTimerbyHandle (Variables|Default|GetRegenerate%20handle))))

(event EventBeginPlay
  ;[1 1 1] Sets the current health to the max at the start of the game
  (Variables|Default|SetCurrentHealth (Variables|Default|GetMaxHealth)))

(fn ChangeHealth
  (params (RegenHealth? :type Boolean) (Amount :type Float%20%28double-precision%29))
  (bind _returnvalue (Math|Float|Absolute(Float) Amount))
  ;[1 1 1] takes the positive amount value and either adds it to current or subtracts it based on if taking damage or healing
  (bind _output_get (Variables|Default|SetCurrentHealth (Math|Float|Clamp(Float) (Math|Float|SelectFloat (+ _returnvalue (Variables|Default|GetCurrentHealth)) (- (Variables|Default|GetCurrentHealth) _returnvalue) RegenHealth?) 0.0 (Variables|Default|GetMaxHealth))))
  ;[1 1 1] Calls the regeneration function on a delay until max health is reached
  (if (< _output_get (Variables|Default|GetMaxHealth))
    (bind _returnvalue_2 (Utilities|Time|SetTimerbyFunctionName 0 "Regenerate Health" (Variables|Default|GetDelay%20between%20regen) true))
    (Variables|Default|SetRegenerate%20handle _returnvalue_2)))