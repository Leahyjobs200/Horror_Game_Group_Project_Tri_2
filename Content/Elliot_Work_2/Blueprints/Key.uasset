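; Key is an interactable pickup that unlocks progress by setting its Door's HasKey flag and advancing the Mannequin to stage 2.
; Interact also plays a door-slam sound at a fixed world location and destroys the key.
; If BP_ObjectiveIncrement's counter matches the key's Index, it updates the player's objective and thoughts, fades the thought text, increments the counter, shows the key icon and sets the respawn location.
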(event EventBeginPlay)

(event Collision|EventActorBeginOverlap
  (params (OtherActor :type Actor%20Object%20Reference)))

(event EventTick
  (params (DeltaSeconds :type Float%20%28single-precision%29)))

(event EventInteract
  (Variables|/Game/Blueprints/David_Work/Blueprints_and_Actors/Door.Door_C|SetHasKey (Variables|Default|GetDoor) true)
  (Variables|/Game/Blueprints/David_Work/Blueprints_and_Actors/JanitorRoom/MannequinDummy.MannequinDummy_C|SetMannequinStage (Variables|Default|GetMannequin) 2)
  (Audio|PlaySoundatLocation "/Game/Sounds/80928__bennstir__door-slam-1.80928__bennstir__door-slam-1" "-2478.000000,2367.000000,148.000000" "0, 0, 0" 1.0 1.0 0.0 0 0 0 0)
  (Actor|DestroyActor)
  (bind _outactors (Actor|GetAllActorsOfClass "/Game/Elliot_Work_2/Blueprints/BP_ObjectiveIncrement.BP_ObjectiveIncrement_C"))
  (bind _asbp_objective_increment (Utilities|Casting|CastToBP_ObjectiveIncrement (Utilities|Array|Get(acopy) _outactors)))
  (if (== (Variables|/Game/Elliot_Work_2/Blueprints/BP_ObjectiveIncrement.BP_ObjectiveIncrement_C|GetIncrement _asbp_objective_increment) (Variables|Default|GetIndex))
    (bind _asbp_first_person_character (Utilities|Casting|CastToBP_FirstPersonCharacter (Game|GetPlayerCharacter 0)))
    (Utilities|FlowControl|DoOnce false
      (:Completed
        (Default|UpdateObjective _asbp_first_person_character (Variables|Default|GetnewObjectiveToSet))
        (Default|UpdateThoughts _asbp_first_person_character (Variables|Default|GetnewThoughtsToSet))
        (bind _newparam (Default|GetPlayerUI _asbp_first_person_character))
        (UserInterface|Animation|PlayAnimation _newparam (Variables|/Game/Elliot_Work_2/HUD/Player_UI.Player_UI_C|GetThoughts_fade _newparam) 0.0 1 "Forward" 1.0 false)
        (Default|Increment+ _asbp_objective_increment)
        (Widget|SetVisibility (Variables|/Game/Elliot_Work_2/HUD/Player_UI.Player_UI_C|GetImage_Key _newparam) "Visible")
        (Variables|/Game/FirstPerson/Blueprints/BP_FirstPersonCharacter.BP_FirstPersonCharacter_C|SetRespawnLocation (.AsBP%20First%20Person%20Character (Utilities|Casting|CastToBP_FirstPersonCharacter (Game|GetPlayerCharacter 0))) (Utilities|Array|Get(acopy) (Variables|/Game/Elliot_Work_2/Blueprints/RespawnPoint.RespawnPoint_C|GetRespawnPoints (Variables|Default|GetRespawnPoint)) (Variables|Default|GetIndex)))))))

(fn ConstructionScript)