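; Trigger volume that switches the lobby lighting to low when its Box is overlapped, optionally advancing the objective.
; With UseIndex set, it fires only while the BP_ObjectiveIncrement actor's Increment matches Index.
; It finds the LightsController by class and calls SetLights.
; If UpdateObjective is set, it passes the new objective and thoughts to TriggerObjective, reusing the actor lookup made only on the UseIndex branch.
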(event OnComponentBeginOverlap(Box)
  (params (OverlappedComponent :type Primitive%20Component%20Object%20Reference) (OtherActor :type Actor%20Object%20Reference) (OtherComp :type Primitive%20Component%20Object%20Reference) (OtherBodyIndex :type Integer) (bFromSweep :type Boolean) (SweepResult :type Hit%20Result%20Structure%20%28by%20ref%29))
  (if (Variables|Default|GetUseIndex?)
    (bind _outactors (Actor|GetAllActorsOfClass "/Game/Elliot_Work_2/Blueprints/BP_ObjectiveIncrement.BP_ObjectiveIncrement_C"))
    (if (== (Variables|Default|Getindex) (Variables|/Game/Elliot_Work_2/Blueprints/BP_ObjectiveIncrement.BP_ObjectiveIncrement_C|GetIncrement (Utilities|Array|Get(acopy) _outactors)))
      (bind _outactors_2 (Actor|GetAllActorsOfClass "/Game/Elliot_Work_2/Blueprints/LightsController.LightsController_C" :!label _label))
      (Default|SetLights (Utilities|Array|Get(acopy) _outactors_2) true false true false false false false false false false false false)
      (if (Variables|Default|GetUpdateObjective?)
        (Default|TriggerObjective (Utilities|Array|Get(acopy) _outactors) (Variables|Default|Getindex) (Variables|Default|GetnewObjectiveToSet) (Variables|Default|GetnewThoughtsToSet) 0 false)))
    (else
      (goto _label))))

(fn ConstructionScript)