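; EntranceDoor is an interactable exit door that returns the player to MainMenuLevel.
; If LiftDoor reports the lobby ready, it opens the menu level immediately.
; Otherwise, once BP_ObjectiveIncrement's count is high enough, it runs a one-time camera fade out and in, triggers the objective, saves through GI_BasicGameInstance and loads the menu.
; Below that count, the player's thoughts UI shows that they can't get out.
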(event EventInteract
  (bind _returnvalue (Game|GetPlayerCameraManager 0))
  (if (Variables|/Game/Blueprints/David_Work/Blueprints_and_Actors/Lift_Stairs.Lift_Stairs_C|GetIsLobbyReady (Variables|Default|GetLiftDoor))
    (Game|OpenLevel(byName) "MainMenuLevel")
    (else
      (bind _outactors (Actor|GetAllActorsOfClass "/Game/Elliot_Work_2/Blueprints/BP_ObjectiveIncrement.BP_ObjectiveIncrement_C"))
      (if (>= (Variables|/Game/Elliot_Work_2/Blueprints/BP_ObjectiveIncrement.BP_ObjectiveIncrement_C|GetIncrement (Utilities|Array|Get(acopy) _outactors)) 13)
        (Utilities|FlowControl|DoOnce false
          (:Completed
            (CameraFades|StartCameraFade :self _returnvalue :ToAlpha 1.0 :Duration 0.5 :bShouldFadeAudio true :bHoldWhenFinished true)
            (Utilities|FlowControl|Delay 0.9)
            (CameraFades|StartCameraFade :self _returnvalue :FromAlpha 1.0 :Duration 0.5 :bShouldFadeAudio true :bHoldWhenFinished true)
            (bind _outactors_2 (Actor|GetAllActorsOfClass "/Game/Elliot_Work_2/Blueprints/BP_ObjectiveIncrement.BP_ObjectiveIncrement_C"))
            (Default|TriggerObjective (Utilities|Array|Get(acopy) _outactors_2) 0 "" "" 0 false)
            (Default|Save (.AsGI%20Basic%20Game%20Instance (Utilities|Casting|CastToGI_BasicGameInstance (Game|GetGameInstance))))
            (Game|OpenLevel(byName) "MainMenuLevel")))
        (else
          (bind _asbp_first_person_character (Utilities|Casting|CastToBP_FirstPersonCharacter (Game|GetPlayerCharacter 0)))
          (Default|UpdateThoughts _asbp_first_person_character "I can't get out!")
          (bind _newparam (Default|GetPlayerUI _asbp_first_person_character))
          (UserInterface|Animation|PlayAnimation _newparam (Variables|/Game/Elliot_Work_2/HUD/Player_UI.Player_UI_C|GetThoughts_fade _newparam) 0.0 1 "Forward" 1.0 false))))))

(fn ConstructionScript)